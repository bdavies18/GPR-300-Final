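; Rake actor that travels along a referenced Track's spline, leaving a trail of static meshes, apparently as rake marks.
; A Path timeline acts as the update driver, turning accumulated time and Speed into spline distance and restarting from zero at the end.
; Every Tick adds a new manually attached mesh at each tine capsule's world location, so components accumulate without cleanup.
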(event Custom|FollowSpline
  (bind _track (Variables|Default|GetTrack))
  (bind _spline (Variables|/Game/Blueprints/RakeSpline.RakeSpline_C|GetSpline _track))
  (Variables|Default|SetDistance 0.0)
  (Variables|Default|SetTime 0.0)
  (Timeline|Path PlayFromStart
    (:Update
      (bind _output_get (Variables|Default|SetTime (+ (Variables|Default|GetTime) (Utilities|Time|GetWorldDeltaSeconds))))
      (Variables|Default|SetDistance (* _output_get (Variables|Default|GetSpeed)))
      (Utilities|IsValid _track
        (:Is%20Valid
          (Transformation|SetActorLocation (Spline|GetLocationatDistanceAlongSpline _spline (Variables|Default|GetDistance) "World") false false)
          (if (>= (Variables|Default|GetDistance) (Spline|GetSplineLength _spline))
            (CallFunction|FollowSpline)))))))

(event EventBeginPlay
  (CallFunction|FollowSpline))

(event Collision|EventActorBeginOverlap
  (params (OtherActor :type Actor%20Object%20Reference)))

(event EventTick
  (params (DeltaSeconds :type Float%20%28single-precision%29))
  (AddComponent|AddStaticMeshComponent true (Math|Conversions|ToTransform(Vector) (Transformation|GetWorldLocation (Variables|Default|GetCapsule))))
  (AddComponent|AddStaticMeshComponent true (Math|Conversions|ToTransform(Vector) (Transformation|GetWorldLocation (Variables|Default|GetCapsule1))))
  (AddComponent|AddStaticMeshComponent true (Math|Conversions|ToTransform(Vector) (Transformation|GetWorldLocation (Variables|Default|GetCapsule2))))
  (AddComponent|AddStaticMeshComponent true (Math|Conversions|ToTransform(Vector) (Transformation|GetWorldLocation (Variables|Default|GetCapsule3))))
  (AddComponent|AddStaticMeshComponent true (Math|Conversions|ToTransform(Vector) (Transformation|GetWorldLocation (Variables|Default|GetCapsule4))))
  (AddComponent|AddStaticMeshComponent true (Math|Conversions|ToTransform(Vector) (Transformation|GetWorldLocation (Variables|Default|GetCapsule5))))
  (AddComponent|AddStaticMeshComponent true (Math|Conversions|ToTransform(Vector) (Transformation|GetWorldLocation (Variables|Default|GetCapsule6))))
  (AddComponent|AddStaticMeshComponent true (Math|Conversions|ToTransform(Vector) (Transformation|GetWorldLocation (Variables|Default|GetCapsule7))))
  (AddComponent|AddStaticMeshComponent true (Math|Conversions|ToTransform(Vector) (Transformation|GetWorldLocation (Variables|Default|GetCapsule8))))
  (AddComponent|AddStaticMeshComponent true (Math|Conversions|ToTransform(Vector) (Transformation|GetWorldLocation (Variables|Default|GetCapsule9))))
  (AddComponent|AddStaticMeshComponent true (Math|Conversions|ToTransform(Vector) (Transformation|GetWorldLocation (Variables|Default|GetCapsule10))))
  (AddComponent|AddStaticMeshComponent true (Math|Conversions|ToTransform(Vector) (Transformation|GetWorldLocation (Variables|Default|GetCapsule11))))
  (AddComponent|AddStaticMeshComponent true (Math|Conversions|ToTransform(Vector) (Transformation|GetWorldLocation (Variables|Default|GetCapsule12)))))

(fn ConstructionScript)